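; BP_EnemyController is an enemy controller Blueprint with logic to track sight of the player through Blackboard keys HasLineOfSight and EnemyActor.
; Sensing a Player-tagged actor clears EnemyTimer and sets both keys, while other sensed actors start that one-shot timer.
; The timer's StartEnemyTimer event resets both keys, whereas a failed sense only prints a message.
; The sensing branch has no triggering event, so it never runs.
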(event `StartEnemyTimer`
  (bind _blackboard (`self.Blackboard`))
  (`BlackboardComponent.SetValueAsBool` _blackboard (`self.HasLineOfSight`) false)
  (`BlackboardComponent.SetValueAsObject` _blackboard (`self.EnemyActor`) null))

(fn `UserConstructionScript`)