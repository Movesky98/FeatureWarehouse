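; BP_Weapon is a weapon item actor that the player can interact with, equip and put down.
; Interact casts the interactor to BP_PlayerCharacter, hands the weapon to its WeaponComponent through SaveWeaponInfo and prints the weapon's name.
; SetupEquipWeapon disables collision on both components and moves the actor to the world origin.
; Putdown detaches it, restores the Item profile on Collision only and places it at the given location.
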(event `/Game/Project/Blueprints/Interfaces/InteractInterface.Interact`
  (params (InteractActor :type "Actor Object Reference"))
  (bind _asbp_player_character (cast `/Game/Project/Blueprints/Gameplay/BP_PlayerCharacter` InteractActor))
  (`/Game/Project/Blueprints/Items/Weapon/Gun/WeaponComponent.SaveWeaponInfo` (`/Game/Project/Blueprints/Gameplay/BP_PlayerCharacter.WeaponComponent` _asbp_player_character) self)
  (`KismetSystemLibrary.PrintString` (`KismetStringLibrary.Concat_StrStr` "Interact Actor Name : " (`KismetSystemLibrary.GetDisplayName` self)) true true (struct :`G` 1.0 :`A` 1.0)))

(fn `Putdown`
  (params (Location :type "Vector Structure"))
  (`self.K2_DetachFromActor` "KeepWorld")
  (`PrimitiveComponent.SetCollisionProfileName` (`self.Collision`) "Item" true)
  (`PrimitiveComponent.SetCollisionProfileName` (`self.SkeletalMesh`) "NoCollision" true)
  (`self.K2_SetActorLocation` (`local.Location`)))

(fn `SetupEquipWeapon`
  (`PrimitiveComponent.SetCollisionProfileName` (`self.Collision`) "NoCollision" true)
  (`PrimitiveComponent.SetCollisionProfileName` (`self.SkeletalMesh`) "NoCollision" true)
  (`self.K2_SetActorLocation` (0.0 0.0 0.0)))

(fn `UserConstructionScript`
  (`parent.UserConstructionScript`))