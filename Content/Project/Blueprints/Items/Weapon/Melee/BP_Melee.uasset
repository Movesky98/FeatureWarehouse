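; BP_Melee is a melee weapon Blueprint that tracks combo attack state and damages BP_Dummy targets with a blade trace.
; On BeginPlay it binds to ABP_Player's montage-end and next-attack-check events, which reset or open the combo window.
; CanAttack allows an attack when idle or when attacking with that window open.
; Start/StopAttackTrace control a looping timer that box-traces between blade sockets, applying fixed damage through the dummy's HealthComponent.
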(event `self.ReceiveBeginPlay`
  (`parent.ReceiveBeginPlay`)
  (`self.BindMontage`))

(fn `AttackTrace`
  (locals (NewLocalVar :type "Array of Actor Object Reference"))
  (bind _skeletalmesh (`self.SkeletalMesh`))
  (bind (_outhit _returnvalue) (`KismetSystemLibrary.BoxTraceSingleForObjects` :`Start` (`SceneComponent.GetSocketLocation` _skeletalmesh "BladeBottom") :`End` (`SceneComponent.GetSocketLocation` _skeletalmesh "BladeTop") :`HalfSize` (3.0 3.0 8.0) :`ObjectTypes` (`|MakeArray` "ObjectTypeQuery9" :!type "EObjectTypeQuery Enum") :`DrawDebugType` "ForDuration" :`DrawTime` 1.0))
  (if _returnvalue
    (bind _asbp_dummy (cast `/Game/Project/Blueprints/Gameplay/BP_Dummy` (`.HitActor` (`GameplayStatics.BreakHitResult` _outhit))))
    (`/Game/Project/Blueprints/Components/HealthComponent.GetDamaged` (`/Game/Project/Blueprints/Gameplay/BP_Dummy.HealthComponent` _asbp_dummy) 30.0)))

(fn `BindMontage`
  (locals (AnimInstance :type "/Game/Project/Animations/ABP_Player Object Reference"))
  (bind _asabp_player (cast `/Game/Project/Animations/ABP_Player` (`SkeletalMeshComponent.GetAnimInstance` (`Character.Mesh` (`GameplayStatics.GetPlayerCharacter` 0)))))
  (bind _output_get (set `local.AnimInstance` _asabp_player))
  (add `AnimInstance.OnMontageEnded` _output_get (`|CreateDelegate` :!event `OnAttackEnded`))
  (add `/Game/Project/Animations/ABP_Player.OnNextAttackCheck` _output_get (`|CreateDelegate` :!event `OnNextAttackChecked`)))

(fn `Can Attack`
  (returns (Result :type Boolean))
  (return (not (xor (`self.CanCombo`) (`self.IsAttacking`)))))

(fn `OnAttackEnded`
  (params (Montage :type "AnimMontage Object Reference") (Interrupted :type Boolean))
  (if (== Montage (`self.AttackMontage`))
    (set `self.MontageIndex` 0)
    (set `self.CanCombo` false)
    (set `self.IsAttacking` false)))

(fn `OnNextAttackChecked`
  (set `self.CanCombo` true))

(fn `StartAttackTrace`
  (bind _returnvalue (`KismetSystemLibrary.K2_SetTimer` null "AttackTrace" 0.01 true))
  (set `self.AttackTraceTimer` _returnvalue))

(fn `StopAttackTrace`
  (`KismetSystemLibrary.K2_ClearAndInvalidateTimerHandle` (`self.AttackTraceTimer`)))

(fn `UserConstructionScript`
  (`parent.UserConstructionScript`))