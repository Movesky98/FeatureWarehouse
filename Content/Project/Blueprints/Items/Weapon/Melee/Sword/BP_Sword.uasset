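; Sword melee weapon Blueprint that performs montage-driven combo attacks on the player character.
; BeginPlay runs the parent logic, then calls BindMontage.
; Attack checks CanAttack, then either starts AttackMontage through BP_PlayerCharacter or, while CanCombo is set, jumps to the section at MontageIndex and clears that flag.
; Both paths advance MontageIndex; a note plans moving the first attack to a C++ wearable-weapon approach.
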(event `self.ReceiveBeginPlay`
  (`parent.ReceiveBeginPlay`)
  (`self.BindMontage`))

(fn `Attack`
  (params (PlayAnimCharacter :type "Character Object Reference"))
  (if (`self.Can Attack`)
    (if (`self.CanCombo`)
      (`AnimInstance.Montage_JumpToSection` (`SkeletalMeshComponent.GetAnimInstance` (`Character.Mesh` (`local.PlayAnimCharacter`))) (`AnimMontage.GetSectionName` (`self.AttackMontage`) (`self.MontageIndex`)) (`self.AttackMontage`))
      (`/Engine/EditorBlueprintResources/StandardMacros.IncrementInt` (`self.MontageIndex`)
        (:`  `
          (set `self.CanCombo` false)))
      (else
        ;[0.02604 0.02604 0.02604 1 13] 첫 공격
        ; 나중에 C++로 구현하면, Weapon Wearable 식으로 구현해서 할 필요가 있음.
        (set `self.IsAttacking` true)
        (bind _asbp_player_character (cast `/Game/Project/Blueprints/Gameplay/BP_PlayerCharacter` (`local.PlayAnimCharacter`)))
        (`/Game/Project/Blueprints/Gameplay/BP_PlayerCharacter.PlayMontage` _asbp_player_character (`self.AttackMontage`))
        (`/Engine/EditorBlueprintResources/StandardMacros.IncrementInt` (`self.MontageIndex`))))))

(fn `UserConstructionScript`
  (`parent.UserConstructionScript`))