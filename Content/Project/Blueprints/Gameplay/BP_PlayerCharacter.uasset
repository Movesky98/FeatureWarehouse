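; Player character Blueprint that maps Enhanced Input to movement, sprinting, crouching, jumping, interaction and weapon use.
; View switching cycles third-person, first-person and top-down by reconfiguring one spring arm, attaching it to the head socket and hiding the head bone for first-person.
; Interaction line-traces from the camera and messages the hit actor.
; WeaponComponent supplies both weapon slots; equipping attaches MainWeapon to a mesh socket and notifies the anim instance, and Attack delegates to that weapon.
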(event `self.ReceiveBeginPlay`
  (switch `/Game/Project/Enums/StateOfViews` (`self.ViewState`)
    (:`NewEnumerator1`
      (`self.SetTPSView`))
    (:`NewEnumerator0`
      (`self.SetFPSView`))
    (:`NewEnumerator2`
      (`self.SetTopView`))))

(event `EnhancedInput|/Game/Project/Inputs/IA_SwitchView`
  (params (ActionValue :type Boolean) (ElapsedSeconds :type "Float (double-precision)") (TriggeredSeconds :type "Float (double-precision)") (InputAction :type "InputAction Object Reference" :default "/Game/Project/Inputs/IA_SwitchView.IA_SwitchView"))
  (:`Triggered`
    (`self.SwitchView`)))

(event `EnhancedInput|/Game/Project/Inputs/IA_MoveForward`
  (params (ActionValue :type "Float (double-precision)") (ElapsedSeconds :type "Float (double-precision)") (TriggeredSeconds :type "Float (double-precision)") (InputAction :type "InputAction Object Reference" :default "/Game/Project/Inputs/IA_MoveForward.IA_MoveForward"))
  ;[0.04688 0.04688 0.04688] Basic Movement
  (:`Triggered`
    (`self.AddMovementInput` (`KismetMathLibrary.GetRightVector` (`SceneComponent.K2_GetComponentRotation` (`self.Mesh`))) ActionValue)))

(event `EnhancedInput|/Game/Project/Inputs/IA_MoveRight`
  (params (ActionValue :type "Float (double-precision)") (ElapsedSeconds :type "Float (double-precision)") (TriggeredSeconds :type "Float (double-precision)") (InputAction :type "InputAction Object Reference" :default "/Game/Project/Inputs/IA_MoveRight.IA_MoveRight"))
  ;[0.04688 0.04688 0.04688] Basic Movement
  (:`Triggered`
    (`self.AddMovementInput` (`KismetMathLibrary.GetForwardVector` (`SceneComponent.K2_GetComponentRotation` (`self.Mesh`))) ActionValue)))

(event `EnhancedInput|/Game/Project/Inputs/IA_Interact`
  (params (ActionValue :type Boolean) (ElapsedSeconds :type "Float (double-precision)") (TriggeredSeconds :type "Float (double-precision)") (InputAction :type "InputAction Object Reference" :default "/Game/Project/Inputs/IA_Interact.IA_Interact"))
  (bind _camera (`self.Camera`))
  (bind _returnvalue (`SceneComponent.K2_GetComponentLocation` _camera))
  (:`Triggered`
    (bind _interactableobject (`self.FindInteractableObject` _returnvalue (+ _returnvalue (* (`SceneComponent.GetForwardVector` _camera) 1000.0))))
    (`/Engine/EditorBlueprintResources/StandardMacros.IsValid` _interactableobject
      (:`Is Valid`
        (message `/Game/Project/Blueprints/Interfaces/InteractInterface.Interact` _interactableobject self)
        (`/Game/Project/Blueprints/Items/Weapon/WeaponComponent.PrintWeaponInfo` (`self.WeaponComponent`))))))

(event `EnhancedInput|/Game/Project/Inputs/IA_Turn`
  (params (ActionValue :type "Float (double-precision)") (ElapsedSeconds :type "Float (double-precision)") (TriggeredSeconds :type "Float (double-precision)") (InputAction :type "InputAction Object Reference" :default "/Game/Project/Inputs/IA_Turn.IA_Turn"))
  ;[0.04688 0.04688 0.04688] Basic Movement
  (:`Triggered`
    (`self.AddControllerYawInput` ActionValue)))

(event `EnhancedInput|/Game/Project/Inputs/IA_LookUp`
  (params (ActionValue :type "Float (double-precision)") (ElapsedSeconds :type "Float (double-precision)") (TriggeredSeconds :type "Float (double-precision)") (InputAction :type "InputAction Object Reference" :default "/Game/Project/Inputs/IA_LookUp.IA_LookUp"))
  ;[0.04688 0.04688 0.04688] Basic Movement
  (:`Triggered`
    (`self.AddControllerPitchInput` ActionValue)))

(event `EnhancedInput|/Game/Project/Inputs/IA_Jump`
  (params (ActionValue :type Boolean) (ElapsedSeconds :type "Float (double-precision)") (TriggeredSeconds :type "Float (double-precision)") (InputAction :type "InputAction Object Reference" :default "/Game/Project/Inputs/IA_Jump.IA_Jump"))
  ;[0.04688 0.04688 0.04688] Basic Movement
  (:`Triggered`
    (if (`self.bIsCrouched`)
      (`self.UnCrouch`)
      (else
        (`self.Jump`)))))

(event `EnhancedInput|/Game/Project/Inputs/IA_SwitchRun`
  (params (ActionValue :type Boolean) (ElapsedSeconds :type "Float (double-precision)") (TriggeredSeconds :type "Float (double-precision)") (InputAction :type "InputAction Object Reference" :default "/Game/Project/Inputs/IA_SwitchRun.IA_SwitchRun"))
  ;[0.04688 0.04688 0.04688] Basic Movement
  (:`Triggered`
    (if ActionValue
      (set `CharacterMovementComponent.MaxWalkSpeed` 600.0 (`self.CharacterMovement`))
      (else
        (set `CharacterMovementComponent.MaxWalkSpeed` 300.0 (`self.CharacterMovement`))))))

(event `EnhancedInput|/Game/Project/Inputs/IA_MainWeapon`
  (params (ActionValue :type Boolean) (ElapsedSeconds :type "Float (double-precision)") (TriggeredSeconds :type "Float (double-precision)") (InputAction :type "InputAction Object Reference" :default "/Game/Project/Inputs/IA_MainWeapon.IA_MainWeapon"))
  (:`Triggered`
    (`self.EquipFirstWeapon`)))

(event `EnhancedInput|/Game/Project/Inputs/IA_Attack`
  (params (ActionValue :type Boolean) (ElapsedSeconds :type "Float (double-precision)") (TriggeredSeconds :type "Float (double-precision)") (InputAction :type "InputAction Object Reference" :default "/Game/Project/Inputs/IA_Attack.IA_Attack"))
  (:`Triggered`
    (`self.Attack`)))

(event `EnhancedInput|/Game/Project/Inputs/IA_Crouch`
  (params (ActionValue :type Boolean) (ElapsedSeconds :type "Float (double-precision)") (TriggeredSeconds :type "Float (double-precision)") (InputAction :type "InputAction Object Reference" :default "/Game/Project/Inputs/IA_Crouch.IA_Crouch"))
  ;[0.04688 0.04688 0.04688] Basic Movement
  (:`Triggered`
    (`/Engine/EditorBlueprintResources/StandardMacros.FlipFlop`
      (:`A`
        (`self.Crouch`))
      (:`B`
        (`self.UnCrouch`)))))

(event `EnhancedInput|/Game/Project/Inputs/IA_SubWeapon`
  (params (ActionValue :type Boolean) (ElapsedSeconds :type "Float (double-precision)") (TriggeredSeconds :type "Float (double-precision)") (InputAction :type "InputAction Object Reference" :default "/Game/Project/Inputs/IA_SubWeapon.IA_SubWeapon"))
  (:`Triggered`
    (`self.EquipSecondWeapon`)))

(fn `Attack`
  (bind _mainweapon (`self.MainWeapon`)
    (:`then`
      (`/Game/Project/Blueprints/Items/Weapon/BP_Weapon.Attack` _mainweapon self))
    (:`else`)))

(fn `EquipFirstWeapon`
  (bind _mainweapon (`self.MainWeapon`))
  (bind _weapon (`/Game/Project/Blueprints/Items/Weapon/WeaponComponent.GetFirstWeapon` (`self.WeaponComponent`)))
  (`/Engine/EditorBlueprintResources/StandardMacros.IsValid` _weapon
    (:`Is Valid`
      (bind _output_get (set `self.MainWeapon` _weapon))
      (if (`|EnumEquality` "NewEnumerator1" (`/Game/Project/Blueprints/Items/Weapon/BP_Weapon.UseType` _output_get))
        (`/Game/Project/Blueprints/Items/Weapon/WeaponComponent.SwapWeapon` (`self.WeaponComponent`) true)
        (`self.K2_AttachToComponent` _mainweapon (`self.Mesh`) (`/Game/Project/Blueprints/Items/Weapon/BP_Weapon.AttachSocketName` _mainweapon) "KeepRelative" "KeepRelative" "KeepRelative" true)
        (`/Game/Project/Blueprints/Items/Weapon/WeaponComponent.NotifyToAnimInstance` (`self.WeaponComponent`))))
    (:`Is Not Valid`
      (`KismetSystemLibrary.PrintString` "PlayerCharacter :: EquipFirstWeapon = There is no first weapon." true true (struct :`R` 1.0 :`A` 1.0)))))

(fn `EquipSecondWeapon`
  (bind _weapon (`/Game/Project/Blueprints/Items/Weapon/WeaponComponent.GetSecondWeapon` (`self.WeaponComponent`)))
  (`/Engine/EditorBlueprintResources/StandardMacros.IsValid` _weapon
    (:`Is Valid`
      (bind _output_get (set `self.MainWeapon` _weapon))
      (if (`|EnumEquality` (`/Game/Project/Blueprints/Items/Weapon/BP_Weapon.UseType` _output_get) "NewEnumerator1")
        (`/Game/Project/Blueprints/Items/Weapon/WeaponComponent.SwapWeapon` (`self.WeaponComponent`) false)
        (`self.K2_AttachToComponent` (`self.MainWeapon`) (`self.Mesh`) (`/Game/Project/Blueprints/Items/Weapon/BP_Weapon.AttachSocketName` (`self.MainWeapon`)) "SnapToTarget" "SnapToTarget" "SnapToTarget" true)
        (`/Game/Project/Blueprints/Items/Weapon/WeaponComponent.NotifyToAnimInstance` (`self.WeaponComponent`))))
    (:`Is Not Valid`
      (`KismetSystemLibrary.PrintString` "PlayerCharacter :: EquipSecondWeapon = There is no second weapon." true true (struct :`R` 1.0 :`A` 1.0)))))

(fn `FindInteractableObject`
  (params (Start :type "Vector Structure") (End :type "Vector Structure"))
  (returns (InteractableObject :type "Actor Object Reference"))
  (bind (_outhit _returnvalue) (`KismetSystemLibrary.LineTraceSingle` :`Start` Start :`End` End :`TraceChannel` "TraceTypeQuery3" :`DrawDebugType` "ForDuration"))
  (if _returnvalue
    (return (`.HitActor` (`GameplayStatics.BreakHitResult` _outhit)))
    (else
      (`KismetSystemLibrary.PrintString` "There is no hit actor."))))

(fn `PlayMontage`
  (params (Animation :type "AnimMontage Object Reference"))
  (bind _asabp_player (cast `/Game/Project/Animations/ABP_Player` (`SkeletalMeshComponent.GetAnimInstance` (`self.Mesh`))))
  (`AnimInstance.Montage_Play` _asabp_player (`local.Animation`) 1.0 "MontageLength" 0.0 true))

(fn `SetFPSView`
  (bind _springarm (`self.SpringArm`))
  (set `self.ViewState` "NewEnumerator0")
  (`SkinnedMeshComponent.HideBoneByName` (`self.Mesh`) "head" "PBO_None")
  (set `SpringArmComponent.bUsePawnControlRotation` true _springarm)
  (bind _returnvalue (`SceneComponent.K2_AttachToComponent` _springarm (`self.Mesh`) "head" "SnapToTarget" "SnapToTarget" "SnapToTarget" true))
  (if _returnvalue
    (`SceneComponent.K2_SetRelativeLocation` _springarm (20.0 0.0 0.0) false false)
    (set `SpringArmComponent.TargetArmLength` 0.0 _springarm)))

(fn `SetTopView`
  (bind _springarm (`self.SpringArm`))
  (set `self.ViewState` "NewEnumerator2")
  (`SkinnedMeshComponent.UnHideBoneByName` (`self.Mesh`) "head")
  (set `SpringArmComponent.bUsePawnControlRotation` false _springarm)
  (bind _returnvalue (`SceneComponent.K2_AttachToComponent` _springarm (`self.Mesh`) "None" "KeepRelative" "KeepRelative" "KeepRelative" true))
  (if _returnvalue
    (`SceneComponent.K2_SetRelativeLocation` _springarm (0.0 0.0 150.0) false false)
    (`SceneComponent.K2_SetRelativeRotation` _springarm (struct :`Pitch` -90.0 :`Yaw` 90.0) false false)
    (set `SpringArmComponent.TargetArmLength` 1000.0 _springarm)))

(fn `SetTPSView`
  (bind _springarm (`self.SpringArm`))
  (set `self.ViewState` "NewEnumerator1")
  (set `SpringArmComponent.bUsePawnControlRotation` true _springarm)
  (`SceneComponent.K2_SetRelativeLocation` _springarm (0.0 0.0 150.0) false false)
  (`SceneComponent.K2_SetRelativeRotation` _springarm (struct :`Yaw` 90.0) false false)
  (set `SpringArmComponent.TargetArmLength` 300.0 _springarm))

(fn `SwitchView`
  (switch `/Game/Project/Enums/StateOfViews` (`self.ViewState`)
    (:`NewEnumerator1`
      (`self.SetFPSView`))
    (:`NewEnumerator0`
      (`self.SetTopView`))
    (:`NewEnumerator2`
      (`self.SetTPSView`))))

(fn `UserConstructionScript`)