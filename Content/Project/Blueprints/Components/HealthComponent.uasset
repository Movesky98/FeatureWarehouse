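; An actor component that tracks health and mana for its owner.
; BeginPlay fills current HP and MP from their maximum values.
; GetDamaged subtracts damage from HP and, at zero or below, only prints a red on-screen message naming the owner as dead.
; MP is never changed after initialisation, and Tick is empty.
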(event `self.ReceiveBeginPlay`
  (set `self.CurHP` (`self.MaxHP`))
  (set `self.CurMP` (`self.MaxMP`)))

(fn `GetDamaged`
  (params (Damage :type "Float (double-precision)"))
  (bind _output_get (set `self.CurHP` (- (`self.CurHP`) Damage)))
  (if (<= _output_get 0.0)
    (`KismetSystemLibrary.PrintString` (`KismetStringLibrary.Concat_StrStr` (`KismetSystemLibrary.GetDisplayName` (`self.GetOwner`)) " is dead.") true true (struct :`R` 1.0 :`A` 1.0))))